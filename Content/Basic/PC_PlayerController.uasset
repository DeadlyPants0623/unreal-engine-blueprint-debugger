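; Player controller for a grid-based building game, handling building placement and selection.
; On BeginPlay it finds the grid manager and creates the building bar and a hidden detail panel.
; Cursor traces on separate channels ease an active preview toward its snapped cell, place its soft class on clicks over clear footprints, or show clicked buildings in the detail panel.
; Debug keys toggle the cursor and recalculate power.
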(event EventBeginPlay
  (bind _returnvalue (Actor|GetActorOfClass "/Game/Engine/GridManager/BP_GridManager.BP_GridManager_C"))
  (Variables|Default|SetGridManagerPtr _returnvalue)
  (bind _returnvalue_2 (UserInterface|CreateWidget "/Game/Blueprint/UI/WBP_BuildingDetail.WBP_BuildingDetail_C" self))
  (Variables|Default|SetBuildingDetailUIPtr _returnvalue_2)
  (UserInterface|Viewport|AddtoViewport _returnvalue_2 1)
  (Widget|SetVisibility _returnvalue_2 "Collapsed")
  (bind _returnvalue_3 (UserInterface|CreateWidget "/Game/Blueprint/UI/WBP_BuildingBar.WBP_BuildingBar_C" self))
  (UserInterface|Viewport|AddtoViewport _returnvalue_3 0)
  (Widget|SetVisibility _returnvalue_3 "Visible"))

(event EventTick
  (params (DeltaSeconds :type Float%20%28single-precision%29))
  (bind (_locationx _locationy) (Game|Player|GetMousePosition))
  (bind _self self)
  (bind _previewactorptr (Variables|Default|GetPreviewActorPtr))
  (bind (_worldposition _worlddirection) (Class|GameplayStatics|DeprojectScreentoWorld _self (Math|Vector2D|MakeVector2D _locationx _locationy)))
  (bind _outhit (Collision|LineTraceByChannel _worldposition (+ _worldposition (* _worlddirection 1e+05)) "TraceTypeQuery4" false 0 "None"))
  (Utilities|IsValid _previewactorptr
    (:Is%20Valid
      (Transformation|SetActorLocation _previewactorptr (Math|Interpolation|Ease "ExpoOut" 0.15 (Transformation|GetActorLocation _previewactorptr) (Default|SnaptoGrid (Variables|Default|GetGridManagerPtr) (.Location (Collision|BreakHitResult _outhit)))) false true))))

(event EventOnStartPreview
  (params (PreviewActorPtr :type Actor%20Object%20Reference))
  (Variables|Default|SetPreviewActorPtr PreviewActorPtr))

(event EventOnEndPreview
  (Variables|Default|SetPreviewActorPtr 0))

(event Input|KeyboardEvents|DebugKeyZ
  (params (Key :type Key%20Structure :default "None") (ActionValue :type Input%20Action%20Value%20Structure))
  (:Pressed
    (bind _isa (Utilities|FlowControl|FlipFlop)
      (:A
        _)
      (:B
        _))
    (Variables|Default|SetbShowMouseCursor _isa)))

(event Input|KeyboardEvents|DebugKeyX
  (params (Key :type Key%20Structure :default "None") (ActionValue :type Input%20Action%20Value%20Structure))
  (:Pressed
    (Default|RecalculatePower (Variables|Default|GetGridManagerPtr))))

(event Input|MouseEvents|LeftMouseButton
  (params (Key :type Key%20Structure :default "None"))
  (bind (_locationx _locationy) (Game|Player|GetMousePosition))
  (bind (_locationx_2 _locationy_2) (Game|Player|GetMousePosition))
  (bind _self self)
  (bind _self_2 self)
  (bind _gridmanagerptr (Variables|Default|GetGridManagerPtr))
  (bind _buildingdetailuiptr (Variables|Default|GetBuildingDetailUIPtr))
  (bind (_worldposition _worlddirection) (Class|GameplayStatics|DeprojectScreentoWorld _self_2 (Math|Vector2D|MakeVector2D _locationx_2 _locationy_2)))
  (bind (_worldposition_2 _worlddirection_2) (Class|GameplayStatics|DeprojectScreentoWorld _self (Math|Vector2D|MakeVector2D _locationx _locationy)))
  (:Pressed
    (Utilities|IsValid (Variables|Default|GetPreviewActorPtr)
      (:Is%20Valid
        (bind (_outhit _returnvalue) (Collision|LineTraceByChannel _worldposition_2 (+ _worldposition_2 (* _worlddirection_2 1e+05)) "TraceTypeQuery4" false 0 "ForDuration"))
        (if _returnvalue
          (if (Default|IsFootprintClear _gridmanagerptr (.Location (Collision|BreakHitResult _outhit)))
            (bind _outval (Class|BPIBuildingPreview|GetSoftPreviewClassPtr(Message) (Variables|Default|GetPreviewActorPtr)))
            (Default|PlaceBuilding _gridmanagerptr (Default|SnaptoGrid (Variables|Default|GetGridManagerPtr) (.Location (Collision|BreakHitResult _outhit))) _outval))))
      (:Is%20Not%20Valid
        (bind (_outhit_2 _returnvalue_2) (Collision|LineTraceByChannel _worldposition (+ _worldposition (* _worlddirection 1e+05)) "TraceTypeQuery3" false 0 "ForDuration"))
        (if _returnvalue_2
          (bind _outval_2 (Class|BPIBuildingBaseGetter|GetGuid(Message) (.HitActor (Collision|BreakHitResult _outhit_2))))
          (Class|BPIBuildingDetailSetter|SetGuid(Message) _buildingdetailuiptr _outval_2)
          (Class|BPIBuildingDetailSetter|SetActorPtr(Message) _buildingdetailuiptr (.HitActor (Collision|BreakHitResult _outhit_2)))
          (Widget|SetVisibility _buildingdetailuiptr "Visible")
          (else
            (Widget|SetVisibility (Variables|Default|GetBuildingDetailUIPtr) "Collapsed")))))))

(fn ConstructionScript)