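; BP_Pylon is a power transmission building that draws cables to the objects it connects to.
; On BeginPlay it binds to its BP_PowerTransmissionComponent's powered and cable-reset events.
; AttachCable, when powered, spawns a cable from the mesh's CableSocket to the connected owner's socket component, with length set to the distance between them.
; OnResetCable destroys cable components under the mesh, running the same loop twice.
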(event `self.ReceiveBeginPlay`
  (bind _returnvalue (`self.GetComponentByClass` "/Game/Blueprint/Buildings/Components/BP_PowerTransmissionComponent.BP_PowerTransmissionComponent_C"))
  (`parent.ReceiveBeginPlay`)
  (add `/Game/Blueprint/Buildings/Components/BP_PowerTransmissionComponent.OnIsPowered` _returnvalue (`|CreateDelegate` :!event `AttachCable`))
  (add `/Game/Blueprint/Buildings/Components/BP_PowerTransmissionComponent.OnResetCable` _returnvalue (`|CreateDelegate` :!event `OnResetCable`)))

(fn `AttachCable`
  (params (bIsPowered :type Boolean) (ConnectedTo :type "ActorComponent Object Reference"))
  (locals (Cable :type "CableComponent Object Reference") (FoundAttached :type Boolean) (Neighbors :type "Array of ActorComponent Object Reference"))
  (bind _cable (`local.Cable`))
  (bind _returnvalue (`ActorComponent.GetOwner` (`local.ConnectedTo`)))
  (if bIsPowered
    (bind _returnvalue_2 (`AddComponent|NODE_AddCableComponent-1` :`bManualAttachment` true))
    (set `local.Cable` _returnvalue_2)
    (`SceneComponent.K2_AttachToComponent` (`local.Cable`) (`self.StaticMesh`) "CableSocket" "SnapToTarget" "SnapToTarget" "SnapToTarget" true)
    (bind _outval (message `/Game/Blueprint/Buildings/Interface/BPI_BuildingBase_Getter.GetCableAttachSocketComponent` _returnvalue))
    (`CableComponent.SetAttachEndToComponent` _cable _outval "CableSocket")
    (set `CableComponent.CableLength` (`KismetMathLibrary.Vector_Distance` (`self.K2_GetActorLocation` self) (`self.K2_GetActorLocation` _returnvalue)) _cable)))

(fn `OnResetCable`
  (for _array_element (`SceneComponent.GetChildrenComponents` (`self.StaticMesh`) true)
    (bind _ascable_component (cast `CableComponent` _array_element))
    (`ActorComponent.K2_DestroyComponent` _ascable_component))
  (for _array_element_2 (`SceneComponent.GetChildrenComponents` (`self.StaticMesh`) true)
    (bind _ascable_component_2 (cast `CableComponent` _array_element_2))
    (`ActorComponent.K2_DestroyComponent` _ascable_component_2)))

(fn `UserConstructionScript`
  (`parent.UserConstructionScript`))