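; Power plant building that visually strings cables to the actors it powers or connects to.
; On BeginPlay it binds an event to its power transmission component's OnIsPowered; AttachCable handles powered connections.
; AttachCable scans the Cube's child cables to avoid duplicates, then spawns a cable from CableSocket to the other actor's interface-provided socket component.
; Cable length comes from the distance to a raised point above that actor.
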(event `self.ReceiveBeginPlay`
  (`parent.ReceiveBeginPlay`)
  (add `/Game/Blueprint/Buildings/Components/BP_PowerTransmissionComponent.OnIsPowered` (`self.GetComponentByClass` "/Game/Blueprint/Buildings/Components/BP_PowerTransmissionComponent.BP_PowerTransmissionComponent_C") (`|CreateDelegate` :!event `AttachCable`)))

(fn `AttachCable`
  (params (bIsPowered :type Boolean) (ConnectedTo :type "ActorComponent Object Reference"))
  (locals (Cable :type "CableComponent Object Reference") (FoundAttached :type Boolean))
  (bind _returnvalue (`ActorComponent.GetOwner` (`local.ConnectedTo`)))
  (if bIsPowered
    (for _array_element (`SceneComponent.GetChildrenComponents` (`self.Cube`) true)
      (bind _ascable_component (cast `CableComponent` _array_element))
      (bind _outval (message `/Game/Blueprint/Buildings/Interface/BPI_BuildingBase_Getter.GetCableAttachSocketComponent` (`ActorComponent.GetOwner` (`local.ConnectedTo`))))
      (if (== (`CableComponent.GetAttachedComponent` _ascable_component) _outval)
        (set `local.FoundAttached` true)))
    (if (not (`local.FoundAttached`))
      (bind _returnvalue_2 (`AddComponent|NODE_AddCableComponent-0` :`bManualAttachment` true))
      (set `local.Cable` _returnvalue_2)
      (`SceneComponent.K2_AttachToComponent` (`local.Cable`) (`self.Cube`) "CableSocket" "SnapToTarget" "SnapToTarget" "SnapToTarget" true)
      (bind _outval_2 (message `/Game/Blueprint/Buildings/Interface/BPI_BuildingBase_Getter.GetCableAttachSocketComponent` _returnvalue))
      (set `CableComponent.CableLength` (`KismetMathLibrary.Vector_Distance` (`self.K2_GetActorLocation` self) (+ (`self.K2_GetActorLocation` _returnvalue) (0.0 0.0 250.0))) (`local.Cable`))
      (`CableComponent.SetAttachEndToComponent` (`local.Cable`) _outval_2 "CableSocket"))))

(fn `UserConstructionScript`
  (`parent.UserConstructionScript`))