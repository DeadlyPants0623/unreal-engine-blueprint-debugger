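; Base actor Blueprint for placeable buildings in a grid-based builder, configured by a Definition data structure.
; On BeginPlay it assigns a GUID, spawns each component class listed in the Definition and passes it generic settings via a message.
; A tick later it registers its footprint with BP_GridManager.
; Getters expose its identity, type, UI tags, cable socket, and tag-found storage and power-transmission components.
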(event `self.ReceiveBeginPlay`
  (set `self.Guid` (`KismetGuidLibrary.NewGuid`))
  (bind _returnvalue (`GameplayStatics.GetActorOfClass` "/Game/Engine/GridManager/BP_GridManager.BP_GridManager_C"))
  (set `self.GridManagerPtr` _returnvalue)
  (`self.AddComponents`)
  (`KismetSystemLibrary.DelayUntilNextTick`)
  (`/Game/Engine/GridManager/BP_GridManager.UpdateFootprint` (`self.GridManagerPtr`) (`self.K2_GetActorLocation`) (`self.Type`) self))

(event `AddComponents`
  (for _array_element (`/Game/Blueprint/Buildings/Components/AutoComponent/BP_BuildingDefinition.Components` (`self.Definition`))
    (bind _asactor_component (castclass `ActorComponent` (`|ConvertAsset` (`.ComponentClass_4_C7F49A6546B342FAE56E39A022027473` (break `/Game/Blueprint/Buildings/Components/AutoComponent/F_BuildingComponentEntry` _array_element)))))
    (bind _returnvalue (`|AddComponentByClass` _asactor_component))
    (message `/Game/Blueprint/Buildings/Components/AutoComponent/BPI_ComponentConfigurable.ApplyGenericSettings` _returnvalue (`.Settings_16_255B8AB545F334DC830BEFB730AFEB09` (break `/Game/Blueprint/Buildings/Components/AutoComponent/F_BuildingComponentEntry` _array_element)))))

(fn `GetCableAttachSocketComponent`
  (returns (OutVal :type "StaticMeshComponent Object Reference"))
  (return (`self.StaticMesh`)))

(fn `GetGuid`
  (returns (OutVal :type "Guid Structure"))
  (return (`self.Guid`)))

(fn `GetPowerTransmissionComponents`
  (returns (OutVal :type "ActorComponent Object Reference"))
  (return (`self.FindComponentByTag` self "/Script/Engine.ActorComponent" "powertransmission")))

(fn `GetRequiredUITags`
  (returns (RV :type "Array of Name"))
  (return (`/Game/Blueprint/Buildings/Components/AutoComponent/BP_BuildingDefinition.RequiredUITags` (`self.Definition`))))

(fn `GetStorageComponent`
  (returns (RV :type "ActorComponent Object Reference"))
  (return (`self.FindComponentByTag` self "/Script/Engine.ActorComponent" "storage")))

(fn `GetType`
  (returns (OutVal :type "/Game/Enum/E_BuildingType Enum"))
  (return (`self.Type`)))

(fn `UserConstructionScript`)