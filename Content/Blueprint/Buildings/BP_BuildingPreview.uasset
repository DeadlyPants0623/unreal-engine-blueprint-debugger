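; Building preview actor that shows a mesh for a selected building type and removes itself once a building is placed.
; On BeginPlay it finds BP_GridManager, binds to its place-building event to destroy itself, and loads its mesh.
; The mesh is looked up by building type in a map, async-loaded and applied to PreviewMesh.
; A getter exposes the soft class reference stored with the preview.
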(event `self.ReceiveBeginPlay`
  (bind _returnvalue (`GameplayStatics.GetActorOfClass` "/Game/Engine/GridManager/BP_GridManager.BP_GridManager_C"))
  (set `self.GridManagerPtr` _returnvalue)
  (add `/Game/Engine/GridManager/BP_GridManager.OnPlaceBuilding` (`self.GridManagerPtr`) (`|CreateDelegate` :!event `OnPlaceBuilding`))
  (`self.LoadStaticMesh`))

(event `LoadStaticMesh`
  (bind _object (`|LoadAsset` (`BlueprintMapLibrary.Map_Find` (`self.PreviewMeshMap`) (`self.PreviewBuildingType`)))
    (:`Completed`
      (bind _asstatic_mesh (cast `StaticMesh` _object))
      (`StaticMeshComponent.SetStaticMesh` (`self.PreviewMesh`) _asstatic_mesh))))

(fn `GetSoftPreviewClassPtr`
  (returns (OutVal :type "Actor Soft Class Reference"))
  (return (`self.PreviewSoftClass`)))

(fn `OnPlaceBuilding`
  (`self.K2_DestroyActor` self))

(fn `UserConstructionScript`)