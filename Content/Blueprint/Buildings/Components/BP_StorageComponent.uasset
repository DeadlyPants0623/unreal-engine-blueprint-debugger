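; Building component that gives its owner a resource storage, handled by the central CRM_StorageManager actor.
; One tick after BeginPlay it finds the manager and registers under the owner's GUID with its storage settings, taken from generic settings.
; Add and remove requests, also exposed as interface-style events, ask the manager whether they are possible before applying them.
; GetResource withdraws the same way and returns whether it succeeded.
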(event `/Game/Blueprint/Buildings/Components/AutoComponent/BPI_ComponentConfigurable.ApplyGenericSettings`
  (params (Settings :type "/Game/Blueprint/Buildings/Components/AutoComponent/F_ComponentSettings_Generic Structure"))
  (set `self.Settings` (`.StorageSetting_33_00FEC77842C6C02D410B4098302A0CAE` (break `/Game/Blueprint/Buildings/Components/AutoComponent/F_ComponentSettings_Generic` Settings))))

(event `self.ReceiveBeginPlay`
  (`KismetSystemLibrary.DelayUntilNextTick`)
  (bind _returnvalue (`GameplayStatics.GetActorOfClass` "/Game/Engine/ComponentsRuntimeManager/CRM_StorageManager.CRM_StorageManager_C"))
  (set `self.StorageManagerPtr` _returnvalue)
  (bind _outval (message `/Game/Blueprint/Buildings/Interface/BPI_BuildingBase_Getter.GetGuid` (`self.GetOwner` self)))
  (set `self.FGuid` _outval)
  (`/Game/Engine/ComponentsRuntimeManager/CRM_StorageManager.CRM_RegisterStorage` (`self.StorageManagerPtr`) (`self.FGuid`) (`self.Settings`)))

(event `AddToStorage`
  (params (ResourceType :type "GameplayTag Structure") (Amount :type Integer))
  (`KismetSystemLibrary.PrintString` (`KismetSystemLibrary.GetDisplayName` (`self.GetOwner`)))
  (if (`/Game/Engine/ComponentsRuntimeManager/CRM_StorageManager.CRM_CanAdd` (`self.StorageManagerPtr`) (`self.FGuid`) ResourceType Amount)
    (`KismetSystemLibrary.PrintString` "can add")
    (`/Game/Engine/ComponentsRuntimeManager/CRM_StorageManager.CRM_AddToStorage` (`self.StorageManagerPtr`) (`self.FGuid`) ResourceType Amount)
    (else
      (`KismetSystemLibrary.PrintString` "cannot add"))))

(event `RemoveFromStorage`
  (params (StorageType :type "GameplayTag Structure") (Amount :type Integer))
  (if (`/Game/Engine/ComponentsRuntimeManager/CRM_StorageManager.CRM_CanGet` (`self.StorageManagerPtr`) (`self.FGuid`) StorageType Amount)
    (`/Game/Engine/ComponentsRuntimeManager/CRM_StorageManager.CRM_GetFromStorage` (`self.StorageManagerPtr`) (`self.FGuid`) StorageType Amount)))

(event `/Game/Blueprint/Buildings/Interface/BPI_Storage.I_AddToStorage`
  (params (ResourceType :type "GameplayTag Structure") (Amount :type Integer))
  (`self.AddToStorage` ResourceType Amount))

(event `/Game/Blueprint/Buildings/Interface/BPI_Storage.I_RemoveFromStorage`
  (params (ResourceType :type "GameplayTag Structure") (Amount :type Integer))
  (`self.RemoveFromStorage` ResourceType Amount))

(fn `GetResource`
  (params (ResourceType :type "GameplayTag Structure") (Amount :type Integer))
  (returns (Success :type Boolean))
  (if (`/Game/Engine/ComponentsRuntimeManager/CRM_StorageManager.CRM_CanGet` (`self.StorageManagerPtr`) (`self.FGuid`) (`local.ResourceType`) (`local.Amount`))
    (`/Game/Engine/ComponentsRuntimeManager/CRM_StorageManager.CRM_GetFromStorage` (`self.StorageManagerPtr`) (`self.FGuid`) (`local.ResourceType`) (`local.Amount`))
    (return true)
    (else
      (return false))))