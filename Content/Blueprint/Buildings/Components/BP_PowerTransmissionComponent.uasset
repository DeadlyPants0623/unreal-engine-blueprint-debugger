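; Building component that makes its owner a node in the power grid, either as a source or a transmitter.
; It takes its transmission settings from generic building settings and exposes range, max transmit count and source status.
; On BeginPlay it finds BP_GridManager and, one tick later, triggers a power recalculation.
; Events update the powered flag and broadcast powered-connection and cable-reset dispatchers.
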(event `/Game/Blueprint/Buildings/Components/AutoComponent/BPI_ComponentConfigurable.ApplyGenericSettings`
  (params (Settings :type "/Game/Blueprint/Buildings/Components/AutoComponent/F_ComponentSettings_Generic Structure"))
  (set `self.Settings` (`.TransmissionSetting_27_DAB8274C4C6FE5F38C3EE3982D6BF5CC` (break `/Game/Blueprint/Buildings/Components/AutoComponent/F_ComponentSettings_Generic` Settings))))

(event `self.ReceiveBeginPlay`
  (bind _returnvalue (`GameplayStatics.GetActorOfClass` "/Game/Engine/GridManager/BP_GridManager.BP_GridManager_C"))
  (set `self.GridManagerPtr` _returnvalue)
  (`KismetSystemLibrary.DelayUntilNextTick`)
  (`/Game/Engine/GridManager/BP_GridManager.RecalculatePower` (`self.GridManagerPtr`)))

(event `/Game/Blueprint/Buildings/Interface/BPI_PowerNode.SetPowered`
  (params (IsPowered :type Boolean))
  (bind _structout (setmembers `/Game/Structure/F_PowerTransmissionSettingsRow` :`StructRef` (`self.Settings`) :`bIsPowered` IsPowered))
  (set `self.Settings` _structout))

(event `/Game/Blueprint/Buildings/Interface/BPI_PowerNode.CallOnPowered`
  (params (bIsPowered :type Boolean) (ConnectedTo :type "ActorComponent Object Reference"))
  (`self.OnIsPowered` bIsPowered ConnectedTo))

(event `/Game/Blueprint/Buildings/Interface/BPI_PowerNode.ResetCable`
  (`self.OnResetCable`))

(fn `GetMaxTransmitAmount`
  (returns (OutVal :type Integer))
  (return (`.MaxTransmitBuilding_9_F7855B904AFECE251FDDA6B359740268` (break `/Game/Structure/F_PowerTransmissionSettingsRow` (`self.Settings`)))))

(fn `GetTransmitRadius`
  (returns (OutVal :type Integer))
  (return (`.Range_5_24AD7A4D44091F32B78669A733965C10` (break `/Game/Structure/F_PowerTransmissionSettingsRow` (`self.Settings`)))))

(fn `IsPowerSource`
  (returns (OutVal :type Boolean))
  (return (`.bIsSource_17_37E1298E44C467C40B1538ABE328994D` (break `/Game/Structure/F_PowerTransmissionSettingsRow` (`self.Settings`)))))