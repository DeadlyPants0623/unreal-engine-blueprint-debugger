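; BP_ResourceProductionComponent is a building component that periodically produces a resource into its owner's storage.
; ApplyGenericSettings takes the production slice of the generic settings, and BeginPlay starts a looping timer at the configured update interval.
; While production is enabled, the update event adds the per-second rate times the interval, rounded, to the owner's BP_StorageComponent through IAddToStorage.
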(event `/Game/Blueprint/Buildings/Components/AutoComponent/BPI_ComponentConfigurable.ApplyGenericSettings`
  (params (Settings :type "/Game/Blueprint/Buildings/Components/AutoComponent/F_ComponentSettings_Generic Structure"))
  (set `self.Settings` (`.ResourceProductionSetting_21_15589BD147C9EC88E2557791C62721CA` (break `/Game/Blueprint/Buildings/Components/AutoComponent/F_ComponentSettings_Generic` Settings))))

(event `self.ReceiveBeginPlay`
  (`KismetSystemLibrary.K2_SetTimerDelegate` (`|CreateDelegate` :!event `UpdateEvent`) (`.UpdateInterval_8_4570ECBB4D6AA0F0C6964E9963FC9D70` (break `/Game/Structure/F_ResourceProductionSettingsRow` (`self.Settings`))) true))

(event `UpdateEvent`
  (bind ((`ResourceType_22_F606811A490A9383840642A7CCDEC8CC` _resourcetype) (`RsourcePerSecond_10_F74041A94EDE096BEED86BA39E344FE4` _rsourcepersecond) (`UpdateInterval_8_4570ECBB4D6AA0F0C6964E9963FC9D70` _updateinterval)) (break `/Game/Structure/F_ResourceProductionSettingsRow` (`self.Settings`)))
  (if (`.bEnabled_5_CE2227074FCA999D33F312B9C53611B6` (break `/Game/Structure/F_ResourceProductionSettingsRow` (`self.Settings`)))
    (`/Game/Blueprint/Buildings/Components/BP_StorageComponent.I_AddToStorage` (`Actor.GetComponentByClass` (`self.GetOwner` self) "/Game/Blueprint/Buildings/Components/BP_StorageComponent.BP_StorageComponent_C") _resourcetype (`KismetMathLibrary.Round` (* _rsourcepersecond _updateinterval)))))