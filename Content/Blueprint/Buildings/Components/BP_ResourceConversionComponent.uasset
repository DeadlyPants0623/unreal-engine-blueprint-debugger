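; BP_ResourceConversionComponent is a building component that periodically converts one resource type into another.
; It takes its conversion settings from the generic settings passed in and starts a looping timer on BeginPlay.
; When enabled, each update requests a fixed input amount from the owner's BP_StorageComponent and, on success, adds the output back to it.
; Output is the per-second rate scaled by the update interval and rounded.
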(event `/Game/Blueprint/Buildings/Components/AutoComponent/BPI_ComponentConfigurable.ApplyGenericSettings`
  (params (Settings :type "/Game/Blueprint/Buildings/Components/AutoComponent/F_ComponentSettings_Generic Structure"))
  (set `self.Settings` (`.ResourceConversionSetting_32_715D128449EDE22BFBBB469CF7C5138E` (break `/Game/Blueprint/Buildings/Components/AutoComponent/F_ComponentSettings_Generic` Settings))))

(event `self.ReceiveBeginPlay`
  (`KismetSystemLibrary.K2_SetTimerDelegate` (`|CreateDelegate` :!event `UpdateEvent`) (`.UpdateInterval_8_4570ECBB4D6AA0F0C6964E9963FC9D70` (break `/Game/Structure/F_ResourceConversionSettingsRow` (`self.Settings`))) true))

(event `UpdateEvent`
  (bind ((`ConvertFrom_15_3F0795B840336585DEF1EFB24AE5B49D` _convertfrom) (`AmountNeeded_20_BAE35AE64E99F1921D4A9C9B99E9DE41` _amountneeded)) (break `/Game/Structure/F_ResourceConversionSettingsRow` (`self.Settings`)))
  (bind ((`ConvertTo_17_3C307131469F65176DB555870EA1493D` _convertto) (`ConversionPerSecond_11_F74041A94EDE096BEED86BA39E344FE4` _conversionpersecond) (`UpdateInterval_8_4570ECBB4D6AA0F0C6964E9963FC9D70` _updateinterval)) (break `/Game/Structure/F_ResourceConversionSettingsRow` (`self.Settings`)))
  (if (`.bEnabled_5_CE2227074FCA999D33F312B9C53611B6` (break `/Game/Structure/F_ResourceConversionSettingsRow` (`self.Settings`)))
    (bind _success (`/Game/Blueprint/Buildings/Components/BP_StorageComponent.GetResource` (`Actor.GetComponentByClass` (`self.GetOwner`) "/Game/Blueprint/Buildings/Components/BP_StorageComponent.BP_StorageComponent_C") _convertfrom _amountneeded))
    (if _success
      (`/Game/Blueprint/Buildings/Components/BP_StorageComponent.AddToStorage` (`Actor.GetComponentByClass` (`self.GetOwner` self) "/Game/Blueprint/Buildings/Components/BP_StorageComponent.BP_StorageComponent_C") _convertto (`KismetMathLibrary.Round` (* _conversionpersecond _updateinterval))))))