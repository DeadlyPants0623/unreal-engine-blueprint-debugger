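; BP_B is an actor in a CustomTest folder that relays branch and switch results to a BP_C actor.
; On BeginPlay it caches the BP_C found in the level.
; FUNC_B branches on a constant true, calls FUNCCTRUE, then switches on an unset building-type value.
; Power Plant and Pylon call FUNCCTRUE again, while Stone Producer, Stone Converter and Residential call FUNCCFALSE, as does the unreachable false branch.
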(event `self.ReceiveBeginPlay`
  (bind _returnvalue (`GameplayStatics.GetActorOfClass` "/Game/CustomTest/BP_C.BP_C_C"))
  (set `self.C` _returnvalue))

(event `FUNC_B`
  (bind _c (`self.C`))
  (bind _c_2 (`self.C`))
  (if true
    (`/Game/CustomTest/BP_C.FUNC_C_TRUE` _c_2)
    (switch `/Game/Enum/E_BuildingType` "NewEnumerator0"
      (:`NewEnumerator1`
        (`/Game/CustomTest/BP_C.FUNC_C_TRUE` _c :!label _label))
      (:`NewEnumerator2`
        (goto _label))
      (:`NewEnumerator3`
        (`/Game/CustomTest/BP_C.FUNC_C_FALSE` _c :!label _label_2))
      (:`NewEnumerator4`
        (goto _label_2))
      (:`NewEnumerator5`
        (goto _label_2)))
    (else
      (`/Game/CustomTest/BP_C.FUNC_C_FALSE` _c_2))))

(fn `UserConstructionScript`)